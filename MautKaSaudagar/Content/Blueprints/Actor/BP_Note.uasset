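; BP_Note is an interactable note actor that shows its text to the player.
; On BeginPlay it caches the player as BaseCharacter; OnInteract copies NoteDescription into that character and calls ShowNote.
; Ending overlap with its Box calls HideNote on the cached character, without checking which actor left.
; IsInteractable always returns true.
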(event OnComponentEndOverlap(Box)
  (params (OverlappedComponent :type Primitive%20Component%20Object%20Reference) (OtherActor :type Actor%20Object%20Reference) (OtherComp :type Primitive%20Component%20Object%20Reference) (OtherBodyIndex :type Integer))
  (Default|HideNote (Variables|Default|GetChar%20Ref)))

(event EventBeginPlay
  (bind _asbase_character (Utilities|Casting|CastToBaseCharacter (Game|GetPlayerCharacter 0)))
  (Variables|Default|SetChar%20Ref _asbase_character))

(event Collision|EventActorBeginOverlap
  (params (OtherActor :type Actor%20Object%20Reference)))

(event EventTick
  (params (DeltaSeconds :type Float%20%28single-precision%29)))

(event EventOnInteract
  (params (Interacting%20Player :type Base%20Character%20Object%20Reference))
  (bind _char_ref (Variables|Default|GetChar%20Ref))
  (Variables|/Game/Core/BaseCharacter.BaseCharacter_C|SetNote _char_ref (Variables|Default|GetNoteDescription))
  (Default|ShowNote _char_ref))

(fn ConstructionScript)

(fn IsInteractable?
  (return true))