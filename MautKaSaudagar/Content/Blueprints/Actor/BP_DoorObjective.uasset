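; Interactable door actor that needs a key and, when opened, gives the player the "Leave The House" objective.
; PickUpKey plays a pickup sound and sets HasKey; interacting without the key prints a hint.
; With the key, OnInteract toggles the OpenCloseDoors timeline forward or in reverse, driving PivotPoint's yaw.
; A DoOnce on the timeline update limits the objective change on the cached player character to one time.
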(event EventBeginPlay
  (bind _asbase_character (Utilities|Casting|CastToBaseCharacter (Game|GetPlayerCharacter 0)))
  (Variables|Default|SetChar%20Ref _asbase_character))

(event Collision|EventActorBeginOverlap
  (params (OtherActor :type Actor%20Object%20Reference)))

(event EventTick
  (params (DeltaSeconds :type Float%20%28single-precision%29)))

(event EventOnInteract
  (params (Interacting%20Player :type Base%20Character%20Object%20Reference))
  (bind _pivotpoint (Variables|Default|GetPivotPoint))
  (bind _relativerotation (Variables|/Script/Engine.SceneComponent|GetRelativeRotation _pivotpoint))
  (if (Variables|Default|GetHasKey?)
    (if (Variables|Default|GetDoorClosed?)
      (Variables|Default|SetDoorClosed? false)
      (bind _alpha (Timeline|OpenCloseDoors Play)
        (:Update
          (Transformation|SetRelativeRotation _pivotpoint (Math|Rotator|MakeRotator (.roll _relativerotation) (.pitch _relativerotation) _alpha) false false)
          (Utilities|FlowControl|DoOnce false
            (:Completed
              (Default|SetObjective (Variables|Default|GetChar%20Ref) "Leave The House")))))
      (else
        (Variables|Default|SetDoorClosed? true)
        (Timeline|OpenCloseDoors Reverse)))
    (else
      (Development|PrintString "You need a key"))))

(event EventPickUpKey
  (Audio|PlaySound2D "/Game/Audio/KeyPickup_Cue.KeyPickup_Cue" 1.0 1.0 0.0 0 0)
  (Variables|Default|SetHasKey? true))

(fn ConstructionScript)

(fn IsInteractable?
  (return true))