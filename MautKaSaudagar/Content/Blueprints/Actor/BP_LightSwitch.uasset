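; BP_LightSwitch is an interactable wall switch actor that toggles the visibility of a referenced Light actor's component.
; On interact, it checks that the light is valid, plays a 2D click sound and flips the light's visibility.
; A timeline plays or reverses to slide the Trigger component along its relative Y axis to match the state.
; It always reports as interactable and caches the player character on BeginPlay.
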(event EventBeginPlay
  (bind _asbase_character (Utilities|Casting|CastToBaseCharacter (Game|GetPlayerCharacter 0)))
  (Variables|Default|SetChar%20Ref _asbase_character))

(event Collision|EventActorBeginOverlap
  (params (OtherActor :type Actor%20Object%20Reference)))

(event EventTick
  (params (DeltaSeconds :type Float%20%28single-precision%29)))

(event EventOnInteract
  (params (Interacting%20Player :type Base%20Character%20Object%20Reference))
  (bind _light (Variables|Default|GetLight))
  (bind _light_2 (Variables|Default|GetLight))
  (bind _trigger (Variables|Default|GetTrigger))
  (bind _lightcomponent (Variables|/Script/Engine.Light|GetLightComponent _light))
  (bind _relativelocation (Variables|/Script/Engine.SceneComponent|GetRelativeLocation _trigger))
  (Utilities|IsValid _light_2
    (:Is%20Valid
      (if (Variables|/Script/Engine.SceneComponent|GetbVisible (Variables|/Script/Engine.Light|GetLightComponent _light_2))
        (Audio|PlaySound2D "/Game/Audio/Flashlight_Switch_Cue.Flashlight_Switch_Cue" 1.0 1.0 0.0 0 0)
        (Rendering|SetVisibility _lightcomponent false false)
        (bind _alpha (Timeline|LightSwitcherAnimation Reverse)
          (:Update
            (Transformation|SetRelativeLocation (Variables|Default|GetTrigger) (Math|Vector|MakeVector (.x _relativelocation) _alpha (.z _relativelocation)) false false)))
        (else
          (Audio|PlaySound2D "/Game/Audio/Flashlight_Switch_Cue.Flashlight_Switch_Cue" 1.0 1.0 0.0 0 0)
          (Rendering|SetVisibility _lightcomponent true false)
          (Timeline|LightSwitcherAnimation Play))))))

(fn ConstructionScript)

(fn IsInteractable?
  (return true))