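; BP_JumpScare is a trigger actor that plays a 2D jump scare sound once.
; The first overlap on its Box component passes a DoOnce and calls the PlayJumpScare event with JumpScareSound, with no check on which actor overlapped.
; BeginPlay caches the player as a BaseCharacter in CharRef, which nothing here uses, and IsInteractable always returns true.
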(event OnComponentBeginOverlap(Box)
  (params (OverlappedComponent :type Primitive%20Component%20Object%20Reference) (OtherActor :type Actor%20Object%20Reference) (OtherComp :type Primitive%20Component%20Object%20Reference) (OtherBodyIndex :type Integer) (bFromSweep :type Boolean) (SweepResult :type Hit%20Result%20Structure%20%28by%20ref%29))
  (Utilities|FlowControl|DoOnce false
    (:Completed
      (CallFunction|PlayJumpScare (Variables|Default|GetJumpScareSound)))))

(event Custom|Play%20JumpScare
  (params (Sound :type Sound%20Base%20Object%20Reference))
  (Audio|PlaySound2D Sound 1.0 1.0 0.0 0 0))

(event EventBeginPlay
  (bind _asbase_character (Utilities|Casting|CastToBaseCharacter (Game|GetPlayerCharacter 0)))
  (Variables|Default|SetChar%20Ref _asbase_character))

(event Collision|EventActorBeginOverlap
  (params (OtherActor :type Actor%20Object%20Reference)))

(event EventTick
  (params (DeltaSeconds :type Float%20%28single-precision%29)))

(fn ConstructionScript)

(fn IsInteractable?
  (return true))