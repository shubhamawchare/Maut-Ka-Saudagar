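; BP_SecondRoomKey is an interactable key pickup for the second room, gated behind the player's third objective.
; It caches the player's BaseCharacter on BeginPlay and always reports itself as interactable.
; On interaction, if Objective3Completed is set, it calls PickUpKey on the referenced doors Blueprint, destroys itself and prints a green "+Key" message.
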(event EventBeginPlay
  (bind _asbase_character (Utilities|Casting|CastToBaseCharacter (Game|GetPlayerCharacter 0)))
  (Variables|Default|SetChar%20Ref _asbase_character))

(event Collision|EventActorBeginOverlap
  (params (OtherActor :type Actor%20Object%20Reference)))

(event EventTick
  (params (DeltaSeconds :type Float%20%28single-precision%29)))

(event EventOnInteract
  (params (Interacting%20Player :type Base%20Character%20Object%20Reference))
  (if (Variables|/Game/Core/BaseCharacter.BaseCharacter_C|GetObjective3Completed? (Variables|Default|GetChar%20Ref))
    (Default|PickUpKey (Variables|Default|GetBP_Doors))
    (Actor|DestroyActor)
    (Development|PrintString "+Key" true true "(R=0.000000,G=1.000000,B=0.116998,A=1.000000)")))

(fn ConstructionScript)

(fn IsInteractable?
  (return true))