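; BP_FlickeringLights is an actor that makes its light component flicker at random intervals.
; The construction script sets the light to its normal intensity.
; From BeginPlay, a looping retriggerable delay waits a random time between MinTime and MaxTime, then a FlipFlop alternates the light between minimum flicker intensity and normal intensity.
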(event EventBeginPlay
  (bind _flickeringlight (Variables|Default|GetFlickeringLight))
  (Utilities|FlowControl|RetriggerableDelay (Math|Random|RandomFloatinRange (Variables|Default|GetMinTime) (Variables|Default|GetMaxTime)) :!label _label)
  (Utilities|FlowControl|FlipFlop
    (:A
      (Rendering|Components|Light|SetIntensity _flickeringlight (Variables|Default|GetMinFlickerIntensity))
      (goto _label))
    (:B
      (Rendering|Components|Light|SetIntensity _flickeringlight (Variables|Default|GetIntensity))
      (goto _label))))

(fn ConstructionScript
  (Rendering|Components|Light|SetIntensity (Variables|Default|GetFlickeringLight) (Variables|Default|GetIntensity)))