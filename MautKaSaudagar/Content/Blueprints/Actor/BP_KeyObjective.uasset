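; BP_KeyObjective is an interactable key pickup that completes the player's first objective.
; On BeginPlay it caches the player as a BaseCharacter.
; When interacted with, it notifies a referenced door through PickUpKey, flags Objective 1 complete, sets the next objective to locate the flickering light, then destroys itself.
; It always reports itself as interactable.
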(event EventBeginPlay
  (bind _asbase_character (Utilities|Casting|CastToBaseCharacter (Game|GetPlayerCharacter 0)))
  (Variables|Default|SetChar%20Ref _asbase_character))

(event Collision|EventActorBeginOverlap
  (params (OtherActor :type Actor%20Object%20Reference)))

(event EventTick
  (params (DeltaSeconds :type Float%20%28single-precision%29)))

(event EventOnInteract
  (params (Interacting%20Player :type Base%20Character%20Object%20Reference))
  (Default|PickUpKey (Variables|Default|GetBP_Doors))
  (Variables|/Game/Core/BaseCharacter.BaseCharacter_C|SetObjective1Completed? (Variables|Default|GetChar%20Ref) true)
  (Default|SetObjective (Variables|Default|GetChar%20Ref) "Locate Flickering Light!")
  (Actor|DestroyActor))

(fn ConstructionScript)

(fn IsInteractable?
  (return true))